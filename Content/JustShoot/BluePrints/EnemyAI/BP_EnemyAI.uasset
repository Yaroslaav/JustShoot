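; BP_EnemyAI is a JustShoot enemy actor with a world-space health bar and death reporting.
; BPCHealth damage events update the healthbar widget as a fraction of max health, and Tick rotates the bar to face the player camera.
; On death it sends killer, victim, gun image and enemy type to the GSB_JustShoot game state, fires its death dispatcher and destroys itself.
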(event `self.ReceiveBeginPlay`
  (bind _bpc_health (`self.BPC_Health`))
  (bind _asgsb_just_shoot (cast `/Game/JustShoot/BluePrints/Game/GSB_JustShoot` (`GameplayStatics.GetGameState`)))
  (set `self.GameStateRef` _asgsb_just_shoot)
  (bind _aswb_healthbar (cast `/Game/JustShoot/Widgets/WB_HealthBar` (`WidgetComponent.GetWidget` (`self.Healthbar`))))
  (`/Game/JustShoot/Widgets/WB_HealthBar.UpdateHealthBar` _aswb_healthbar 1.0)
  (add `/Game/JustShoot/BluePrints/Health/BPC_Health.OnDamage` _bpc_health (delegate `OnDamage`))
  (add `/Game/JustShoot/BluePrints/Health/BPC_Health.OnDeath` _bpc_health (delegate `Death`)))

(event `OnDamage`
  (params (CurrentHealth :type "Float (double-precision)"))
  (`self.OnReciveDamage` CurrentHealth (stale `self.ReceiveBeginPlay` _aswb_healthbar)))

(event `Death`
  (params (DamagerName :type Text) (GunImage :type "Texture2D Object Reference"))
  (`self.Die` DamagerName GunImage))

(event `self.ReceiveTick`
  (params (DeltaSeconds :type "Float (single-precision)"))
  (bind _healthbar (`self.Healthbar`))
  (`SceneComponent.K2_SetWorldRotation` _healthbar (`KismetMathLibrary.FindLookAtRotation` (`SceneComponent.K2_GetComponentLocation` _healthbar) (`SceneComponent.K2_GetComponentLocation` (`PlayerCameraManager.TransformComponent` (`GameplayStatics.GetPlayerCameraManager` 0)))) false false))

(fn `Die`
  (params (KillerName :type Text) (GunImage :type "Texture2D Object Reference"))
  (`/Game/JustShoot/BluePrints/Game/GSB_JustShoot.SmbDie` (`self.GameStateRef`) (make `/Game/JustShoot/BluePrints/BPS_SmbDiedInfo` KillerName (`KismetTextLibrary.Conv_StringToText` (`KismetSystemLibrary.GetDisplayName` self)) GunImage (`self.EnemyType`)))
  (`self.OnDeath`)
  (`self.K2_DestroyActor`))

(fn `OnReciveDamage`
  (params (Damage :type "Float (double-precision)") (Target :type "/Game/JustShoot/Widgets/WB_HealthBar Object Reference"))
  (`/Game/JustShoot/Widgets/WB_HealthBar.UpdateHealthBar` Target (/ Damage (`/Game/JustShoot/BluePrints/Health/BPC_Health.MaxHealth` (`self.BPC_Health`)))))

(fn `UserConstructionScript`)