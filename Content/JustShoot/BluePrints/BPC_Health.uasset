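; BPC_Health is the health component for JustShoot, tracking current and max health and exposing getters for both.
; BeginPlay fills health to max and caches the GSB_JustShoot game state, printing its name.
; Damage subtracts health, broadcasts OnDamage and calls Die at zero or below.
; Die reports to the game state's SmbDie, passing the component's own name as killer and the damager's as killed, then broadcasts OnDeath.
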(event `self.ReceiveBeginPlay`
  (set `self.CurrentHealth` (`self.MaxHealth`))
  (bind _asgsb_just_shoot (cast `/Game/JustShoot/BluePrints/Game/GSB_JustShoot` (`GameplayStatics.GetGameState`)))
  (bind _output_get (set `self.GameStateRef` _asgsb_just_shoot))
  (`KismetSystemLibrary.PrintString` (`KismetSystemLibrary.GetDisplayName` _output_get)))

(fn `Damage`
  (params (Damage :type "Float (double-precision)") (DamagerName :type Text) (GunType :type Text))
  (bind _output_get (set `self.CurrentHealth` (- (`self.CurrentHealth`) Damage)))
  (`self.OnDamage` _output_get)
  (if (<= _output_get 0.0)
    (`self.Die` DamagerName GunType)))

(fn `Die`
  (params (DamagerName :type Text) (GunType :type Text))
  (`/Game/JustShoot/BluePrints/Game/GSB_JustShoot.SmbDie` (`self.GameStateRef`) (`KismetTextLibrary.Conv_StringToText` (`KismetSystemLibrary.GetDisplayName` self)) DamagerName GunType)
  (`self.OnDeath`))

(fn `GetCurrentHealth`
  (returns (health :type "Float (double-precision)"))
  (return (`self.CurrentHealth`)))

(fn `GetMaxHealth`
  (returns (MaxHealth :type "Float (double-precision)"))
  (return (`self.MaxHealth`)))