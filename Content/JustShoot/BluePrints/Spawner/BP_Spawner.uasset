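; BP_Spawner is an enemy spawner that fills the level up to MaxSpawnedEnemiesAmount on BeginPlay and replenishes it as enemies die.
; Spawn loops until the cap is reached, placing each enemy at a random SpawnPoints location and binding its OnDeath event to refill the count.
; GetEnemy does a weighted pick, treating Enemies map keys as percentage thresholds and choosing the closest one at or below a random roll.
; SpawnBoss is an empty stub.
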(event `self.ReceiveBeginPlay`
  (`self.Spawn`))

(event `SpawnBoss`)

(fn `GetEnemy`
  (returns (Enemy :type "/Game/JustShoot/BluePrints/EnemyAI/BP_EnemyAI Class Reference"))
  (locals (Percent :type "Float (double-precision)" :default 0.0) (MinDifference :type "Float (double-precision)") (ChosenIndex :type Integer))
  (bind _percent (`local.Percent`))
  (set `local.MinDifference` 100.0)
  (set `local.Percent` (`KismetMathLibrary.RandomFloatInRange` 0.0 101.0))
  (for _index (range (+ (`BlueprintMapLibrary.Map_Length` (`self.Enemies`)) 1))
    (bind _keys (`BlueprintMapLibrary.Map_Keys` (`self.Enemies`)))
    (bind _output (`|GetArrayItem` _keys _index))
    (bind _returnvalue (`KismetMathLibrary.Abs` (- _percent _output)))
    (if (and (<= _output _percent) (< _returnvalue (`local.MinDifference`)))
      (set `local.ChosenIndex` _index)
      (set `local.MinDifference` _returnvalue)))
  (bind _values (`BlueprintMapLibrary.Map_Values` (`self.Enemies`)))
  (return (`|GetArrayItem` _values (`local.ChosenIndex`))))

(fn `GetRandomSpawnPoint`
  (returns (Postion :type "Vector Structure"))
  (return (`|GetArrayItem` (`self.SpawnPoints`) (`KismetMathLibrary.RandomInteger` (`KismetArrayLibrary.Array_Length` (`self.SpawnPoints`))))))

(fn `OnSpawnedEnemyDie`
  (bind _result (`/Engine/EditorBlueprintResources/StandardMacros.DecrementInt` (`self.SpawnedEnemies`))
    (:`  `
      (set `self.SpawnedEnemies` _result)
      (`self.Spawn`))))

(fn `Spawn`
  (while (< (`self.SpawnedEnemies`) (`self.MaxSpawnedEnemiesAmount`))
    (bind _postion (`self.GetRandomSpawnPoint`))
    (bind _enemy (`self.GetEnemy`))
    (bind _returnvalue (`|SpawnActorFromClass` _enemy (`KismetMathLibrary.MakeTransform` _postion) "Undefined" "MultiplyWithRoot" null null))
    (`/Engine/EditorBlueprintResources/StandardMacros.IsValid` _returnvalue
      (:`Is Valid`
        (bind _result (`/Engine/EditorBlueprintResources/StandardMacros.IncrementInt` (`self.SpawnedEnemies`))
          (:`  `
            (set `self.SpawnedEnemies` _result)
            (add `/Game/JustShoot/BluePrints/EnemyAI/BP_EnemyAI.OnDeath` _returnvalue (`|CreateDelegate` :!event `OnSpawnedEnemyDie`))))))))

(fn `UserConstructionScript`)