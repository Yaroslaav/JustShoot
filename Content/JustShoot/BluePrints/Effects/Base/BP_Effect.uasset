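; BP_Effect is a base component for timed effects in JustShoot.
; SetInfo stores the effect info and starts a lifetime timer that Tick accumulates from delta seconds.
; When the timer reaches the lifetime in the effect data, it broadcasts OnEffectEnd with the info and destroys the component.
; RemoveEffect runs the same end-and-destroy sequence immediately, without waiting for expiry.
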(event `self.ReceiveBeginPlay`)

(event `self.ReceiveTick`
  (params (DeltaSeconds :type "Float (single-precision)"))
  (if (`self.CanStartDestroyTimer`)
    (bind _output_get (set `self.LifeTime` (+ DeltaSeconds (`self.LifeTime`))))
    (if (>= _output_get (`/Game/JustShoot/BluePrints/Effects/Base/PDA_Effect.LifeTime` (`.EffectData_26_90F7F42D40C2217B45C08CAE9E69DC76` (break `/Game/JustShoot/BluePrints/Effects/Miscellaneous/S_EffectInfo` (`self.Info`)))))
      (`self.OnEffectEnd` (`self.Info`))
      (`self.K2_DestroyComponent`))))

(fn `RemoveEffect`
  (`self.OnEffectEnd` (`self.Info`))
  (`self.K2_DestroyComponent`))

(fn `SetInfo`
  (params (Info :type "/Game/JustShoot/BluePrints/Effects/Miscellaneous/S_EffectInfo Structure"))
  (set `self.Info` Info)
  (set `self.CanStartDestroyTimer` true))