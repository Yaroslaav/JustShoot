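; BP_CustomMovement is a movement component for pawns that forwards walk and jump input and applies timed walk-speed and jump-boost effects.
; On begin play it finds the owner's CharacterMovement component and sets normal walk speed and jump velocity.
; Each boost spawns an effect component, tags the owner and multiplies the base value, replacing any existing effect found by that tag.
; Remove functions restore normal values and clear the tag.
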(event `self.ReceiveBeginPlay`
  (`self.Setup`))

(fn `ApplyJumpBoostEffect`
  (params (Info :type "/Game/JustShoot/BluePrints/Effects/Miscellaneous/S_EffectInfo Structure"))
  (returns (Effect :type "/Game/JustShoot/BluePrints/Effects/Base/BP_Effect Object Reference"))
  (bind (_spawnchance _effectdata) (break `/Game/JustShoot/BluePrints/Effects/Miscellaneous/S_EffectInfo` Info))
  (bind _owner (`self.Owner`))
  (bind _effect (`/Game/JustShoot/BluePrints/Effects/Base/PDA_Effect.Effect` _effectdata))
  (bind _effecttagname (`/Game/JustShoot/BluePrints/Effects/Base/PDA_Effect.EffectTagName` _effectdata))
  (bind (_containceeffect _foundeffect) (`self.CheckEffect` _effecttagname _effect))
  (if _containceeffect
    (`KismetSystemLibrary.PrintString` "Why")
    (`/Game/JustShoot/BluePrints/Effects/Base/BP_Effect.RemoveEffect` _foundeffect))
  (bind _returnvalue (`|AddComponentByClass` _owner _effect))
  (`KismetArrayLibrary.Array_Add` (`Actor.Tags` _owner) _effecttagname)
  (`/Game/JustShoot/BluePrints/Effects/Base/BP_Effect.SetInfo` _returnvalue Info)
  (bind _output_get (set `self.JumpMultiplier` (`/Game/JustShoot/BluePrints/Effects/Base/PDA_Effect.Value` _effectdata)))
  (bind _output_get_2 (set `self.JumpVelocity` (* _output_get (`self.NormalJumpVelocity`))))
  (set `CharacterMovementComponent.JumpZVelocity` _output_get_2 (`self.CharacterMovement`))
  (add `/Game/JustShoot/BluePrints/Effects/Base/BP_Effect.OnEffectEnd` _returnvalue (`|CreateDelegate` :!event `RemoveJumpBoost`))
  (return _returnvalue))

(fn `ApplyWalkSpeedUpEffect`
  (params (EffectInfo :type "/Game/JustShoot/BluePrints/Effects/Miscellaneous/S_EffectInfo Structure"))
  (returns (Effect :type "/Game/JustShoot/BluePrints/Effects/Base/BP_Effect Object Reference"))
  (bind (_spawnchance _effectdata) (break `/Game/JustShoot/BluePrints/Effects/Miscellaneous/S_EffectInfo` EffectInfo))
  (bind _owner (`self.Owner`))
  (bind _effect (`/Game/JustShoot/BluePrints/Effects/Base/PDA_Effect.Effect` _effectdata))
  (bind _effecttagname (`/Game/JustShoot/BluePrints/Effects/Base/PDA_Effect.EffectTagName` _effectdata))
  (bind (_containceeffect _foundeffect) (`self.CheckEffect` _effecttagname _effect))
  (if _containceeffect
    (`/Game/JustShoot/BluePrints/Effects/Base/BP_Effect.RemoveEffect` _foundeffect))
  (bind _returnvalue (`|AddComponentByClass` _owner _effect))
  (`KismetArrayLibrary.Array_Add` (`Actor.Tags` _owner) _effecttagname)
  (`/Game/JustShoot/BluePrints/Effects/Base/BP_Effect.SetInfo` _returnvalue EffectInfo)
  (bind _output_get (set `self.MovementMultiplier` (`/Game/JustShoot/BluePrints/Effects/Base/PDA_Effect.Value` _effectdata)))
  (bind _output_get_2 (set `self.MaxWalkSpeed` (* _output_get (`self.NormalWalkSpeed`))))
  (set `CharacterMovementComponent.MaxWalkSpeed` _output_get_2 (`self.CharacterMovement`))
  (add `/Game/JustShoot/BluePrints/Effects/Base/BP_Effect.OnEffectEnd` _returnvalue (`|CreateDelegate` :!event `RemoveSpeedBoost`))
  (return _returnvalue))

(fn `CheckEffect`
  (params (Tag :type Name) (Effect :type "/Game/JustShoot/BluePrints/Effects/Base/BP_Effect Class Reference"))
  (returns (ContainceEffect :type Boolean) (FoundEffect :type "/Game/JustShoot/BluePrints/Effects/Base/BP_Effect Object Reference"))
  (bind _owner (`self.Owner`))
  (if (`Actor.ActorHasTag` _owner Tag)
    (return true (`Actor.GetComponentByClass` _owner Effect))
    (else
      (return false null))))

(fn `Jump`
  (bind _ascharacter (cast `Character` (`self.Owner`)))
  (`Character.Jump` _ascharacter))

(fn `RemoveJumpBoost`
  (params (Info :type "/Game/JustShoot/BluePrints/Effects/Miscellaneous/S_EffectInfo Structure"))
  (set `self.JumpMultiplier` 1.0)
  (bind _output_get (set `CharacterMovementComponent.JumpZVelocity` (`self.NormalJumpVelocity`) (`self.CharacterMovement`)))
  (set `self.JumpVelocity` _output_get)
  (`KismetArrayLibrary.Array_RemoveItem` (`Actor.Tags` (`self.Owner`)) (`/Game/JustShoot/BluePrints/Effects/Base/PDA_Effect.EffectTagName` Info_EffectData_26_90F7F42D40C2217B45C08CAE9E69DC76)))

(fn `RemoveSpeedBoost`
  (params (Info :type "/Game/JustShoot/BluePrints/Effects/Miscellaneous/S_EffectInfo Structure"))
  (set `self.MovementMultiplier` 1.0)
  (bind _output_get (set `CharacterMovementComponent.MaxWalkSpeed` (`self.NormalWalkSpeed`) (`self.CharacterMovement`)))
  (set `self.MaxWalkSpeed` _output_get)
  (`KismetArrayLibrary.Array_RemoveItem` (`Actor.Tags` (`self.Owner`)) (`/Game/JustShoot/BluePrints/Effects/Base/PDA_Effect.EffectTagName` Info_EffectData_26_90F7F42D40C2217B45C08CAE9E69DC76)))

(fn `Setup`
  (bind _aspawn (cast `Pawn` (`self.GetOwner`))
    (:`then`
      (bind _output_get (set `self.Owner` _aspawn))
      (bind _returnvalue (`Actor.GetComponentByClass` _output_get "/Script/Engine.CharacterMovementComponent"))
      (`/Engine/EditorBlueprintResources/StandardMacros.IsValid` _returnvalue
        (:`Is Valid`
          (bind _output_get_2 (set `self.CharacterMovement` _returnvalue))
          (bind _output_get_3 (set `CharacterMovementComponent.MaxWalkSpeed` (`self.NormalWalkSpeed`) _output_get_2))
          (set `self.MaxWalkSpeed` _output_get_3)
          (bind _output_get_4 (set `CharacterMovementComponent.JumpZVelocity` (`self.NormalJumpVelocity`) _output_get_2))
          (set `self.JumpVelocity` _output_get_4))
        (:`Is Not Valid`
          (`AutomationBlueprintFunctionLibrary.AddExpectedLogError` "You can`t use movement component on this actor"))))
    (:`CastFailed`
      (`AutomationBlueprintFunctionLibrary.AddExpectedLogError` "You can`t use movement component on this actor"))))

(fn `SetWalkMovementInput`
  (params (WorldDirection :type "Vector Structure") (ScaleValue :type "Float (double-precision)") (Force :type Boolean))
  (`Pawn.AddMovementInput` (`self.Owner`) WorldDirection ScaleValue Force))

(fn `StopJumping`
  (bind _ascharacter (cast `Character` (`self.Owner`)))
  (`Character.StopJumping` _ascharacter))