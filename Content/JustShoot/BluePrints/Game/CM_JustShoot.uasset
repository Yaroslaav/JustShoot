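; Cheat manager for JustShoot, with debug commands that apply effects to the first-person player character.
; Speed and jump boost commands build a row name from effect type and level, while a generic command takes the name directly.
; Each looks up DT_EffectsInfo, passes a found row to ApplyEffect on player 0's BP_FirstPersonCharacter, and prints whether the lookup succeeded.
; SpawnBosss is a stub that only prints a test string.
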(fn `AddEffectToPlayer`
  (params (Name :type Name))
  (bind _returnvalue (`KismetStringLibrary.Conv_NameToString` Name))
  (bind _returnvalue_2 (`|GetDataTableRow` "/Game/JustShoot/BluePrints/Effects/Miscellaneous/DT_EffectsInfo.DT_EffectsInfo" Name)
    (:`then`
      (`KismetSystemLibrary.PrintString` (`KismetStringLibrary.Concat_StrStr` "Add " _returnvalue))
      (bind _asbp_first_person_character (cast `/Game/FirstPerson/Blueprints/BP_FirstPersonCharacter` (`GameplayStatics.GetPlayerCharacter` 0)))
      (`/Game/FirstPerson/Blueprints/BP_FirstPersonCharacter.ApplyEffect` _asbp_first_person_character _returnvalue_2))
    (:`RowNotFound`
      (`KismetSystemLibrary.PrintString` (`KismetStringLibrary.Concat_StrStr` "Fail to add  " _returnvalue)))))

(fn `AddJumpBoosteffectToPlayer`
  (params (Level :type Integer))
  (bind _returnvalue (`KismetStringLibrary.Concat_StrStr` "JumpBoost" (`KismetStringLibrary.Conv_IntToString` Level)))
  (bind _returnvalue_2 (`|GetDataTableRow` "/Game/JustShoot/BluePrints/Effects/Miscellaneous/DT_EffectsInfo.DT_EffectsInfo" (`KismetStringLibrary.Conv_StringToName` _returnvalue))
    (:`then`
      (`KismetSystemLibrary.PrintString` (`KismetStringLibrary.Concat_StrStr` "Add " _returnvalue))
      (bind _asbp_first_person_character (cast `/Game/FirstPerson/Blueprints/BP_FirstPersonCharacter` (`GameplayStatics.GetPlayerCharacter` 0)))
      (`/Game/FirstPerson/Blueprints/BP_FirstPersonCharacter.ApplyEffect` _asbp_first_person_character _returnvalue_2))
    (:`RowNotFound`
      (`KismetSystemLibrary.PrintString` (`KismetStringLibrary.Concat_StrStr` "Fail to add  " _returnvalue)))))

(fn `AddSpeedBoostEffectToPlayer`
  (params (Level :type Integer))
  (bind _returnvalue (`KismetStringLibrary.Concat_StrStr` "SpeedBoost" (`KismetStringLibrary.Conv_IntToString` Level)))
  (`KismetSystemLibrary.PrintString` (`KismetStringLibrary.Conv_IntToString` Level) true true (struct :`G` 1.0 :`B` 0.372354 :`A` 1.0))
  (bind _returnvalue_2 (`|GetDataTableRow` "/Game/JustShoot/BluePrints/Effects/Miscellaneous/DT_EffectsInfo.DT_EffectsInfo" (`KismetStringLibrary.Conv_StringToName` _returnvalue))
    (:`then`
      (`KismetSystemLibrary.PrintString` (`KismetStringLibrary.Concat_StrStr` "Add " _returnvalue))
      (bind _asbp_first_person_character (cast `/Game/FirstPerson/Blueprints/BP_FirstPersonCharacter` (`GameplayStatics.GetPlayerCharacter` 0)))
      (`/Game/FirstPerson/Blueprints/BP_FirstPersonCharacter.ApplyEffect` _asbp_first_person_character _returnvalue_2))
    (:`RowNotFound`
      (`KismetSystemLibrary.PrintString` (`KismetStringLibrary.Concat_StrStr` "Fail to add  " _returnvalue)))))

(fn `SpawnBosss`
  (`KismetSystemLibrary.PrintString` "Hello"))