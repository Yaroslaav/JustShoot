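; Health component for JustShoot that tracks an actor's current and maximum health.
; On BeginPlay it fills health to maximum and caches the GSB_JustShoot game state, which is not otherwise used in these graphs.
; Damage subtracts health without clamping and broadcasts OnDamage with the new value.
; At zero or below, Die broadcasts OnDeath with the damager's name and gun image, with no guard against repeated deaths.
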(event `self.ReceiveBeginPlay`
  (set `self.CurrentHealth` (`self.MaxHealth`))
  (bind _asgsb_just_shoot (cast `/Game/JustShoot/BluePrints/Game/GSB_JustShoot` (`GameplayStatics.GetGameState`)))
  (set `self.GameStateRef` _asgsb_just_shoot))

(fn `Damage`
  (params (Damage :type "Float (double-precision)") (DamagerName :type Text) (GunImage :type "Texture2D Object Reference"))
  (bind _output_get (set `self.CurrentHealth` (- (`self.CurrentHealth`) Damage)))
  (`self.OnDamage` _output_get)
  (if (<= _output_get 0.0)
    (`self.Die` DamagerName GunImage)))

(fn `Die`
  (params (DamagerName :type Text) (GunImage :type "Texture2D Object Reference"))
  (`self.OnDeath` DamagerName GunImage))

(fn `GetCurrentHealth`
  (returns (health :type "Float (double-precision)"))
  (return (`self.CurrentHealth`)))

(fn `GetMaxHealth`
  (returns (MaxHealth :type "Float (double-precision)"))
  (return (`self.MaxHealth`)))