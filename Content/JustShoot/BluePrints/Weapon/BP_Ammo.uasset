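; BP_Ammo is a weapon ammo Blueprint that tracks the current round count and handles reloading.
; ReduceAmmo subtracts the per-shot cost and triggers Reload when ammo runs out with auto-reload enabled.
; Reload sets the Reloading flag, broadcasts reload start and refills to max immediately, with no delay.
; The reload-end broadcast is unconnected, and nothing here clears the Reloading flag.
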(fn `ReduceAmmo`
  (bind _output_get (set `self.CurrentAmmo` (- (`self.CurrentAmmo`) (`self.AmmoPerShot`))))
  (if (and (<= _output_get 0) (`self.AutoReload`))
    (`self.Reload`)))

(fn `Reload`
  (set `self.Reloading` true)
  (`self.OnReloadingStart`)
  (set `self.CurrentAmmo` (`self.MaxAmmo`)))